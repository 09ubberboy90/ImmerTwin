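; Kinematic UR3 robot arm with an attached Robotiq 2F-85 gripper, assembled entirely in the construction script.
; Registers base-to-wrist meshes as links, then chains six joints between consecutive links by array index.
; Link and joint names derive from component names converted to snake_case, so component naming matters.
; The gripper child actor is cached and set as the robot of its own ROS2 interface.
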(fn `UserConstructionScript`
  (bind _linkmeshes (`self.linkmeshes`))
  (bind _linkmeshes_2 (`self.linkmeshes`))
  (bind _rrjoints (`self.RRjoints`))
  (`|ExecutionSequence`
    (:`then_0`
      (`KismetArrayLibrary.Array_Clear` (`self.linkmeshes`))
      (`KismetArrayLibrary.Array_Clear` (`self.RRjoints`)))
    (:`then_1`
      (`KismetArrayLibrary.Array_Add` _linkmeshes_2 (`self.Base`))
      (`KismetArrayLibrary.Array_Add` _linkmeshes_2 (`self.Shoulder`))
      (`KismetArrayLibrary.Array_Add` _linkmeshes_2 (`self.Upper`))
      (`KismetArrayLibrary.Array_Add` _linkmeshes_2 (`self.Forearm`))
      (`KismetArrayLibrary.Array_Add` _linkmeshes_2 (`self.Wrist1`))
      (`KismetArrayLibrary.Array_Add` _linkmeshes_2 (`self.Wrist2`))
      (`KismetArrayLibrary.Array_Add` _linkmeshes_2 (`self.Wrist3`))
      (for _array_element (`self.linkmeshes`)
        (`self.AddLink` (`RRGeneralUtils.PascalToSnake` (`KismetSystemLibrary.GetObjectName` _array_element)) _array_element)))
    (:`then_2`
      (`KismetArrayLibrary.Array_Add` _rrjoints (`self.ShoulderPanJoint`))
      (`KismetArrayLibrary.Array_Add` _rrjoints (`self.ShoulderLiftJoint`))
      (`KismetArrayLibrary.Array_Add` _rrjoints (`self.ElbowJoint`))
      (`KismetArrayLibrary.Array_Add` _rrjoints (`self.Wrist1Joint`))
      (`KismetArrayLibrary.Array_Add` _rrjoints (`self.Wrist2Joint`))
      (`KismetArrayLibrary.Array_Add` _rrjoints (`self.Wrist3Joint`))
      (for (_array_element_2 _array_index) (`self.RRjoints`)
        (`self.AddJoint` (`RRGeneralUtils.PascalToSnake` (`KismetSystemLibrary.GetObjectName` (`|GetArrayItem` _linkmeshes _array_index))) (`RRGeneralUtils.PascalToSnake` (`KismetSystemLibrary.GetObjectName` (`|GetArrayItem` _linkmeshes (+ _array_index 1)))) (`RRGeneralUtils.PascalToSnake` (`KismetSystemLibrary.GetObjectName` _array_element_2) true) _array_element_2)))
    (:`then_3`
      (bind _asrobotiq_2f_85_base_blueprint (cast `/Game/Ur3/Robotiq_2f85/Robotiq_2F_85_base_Blueprint` (`ChildActorComponent.ChildActor` (`self.gripper`))))
      (bind _output_get (set `self.GripperActor` _asrobotiq_2f_85_base_blueprint))
      (set `RRRobotROS2Interface.Robot` _output_get (`RRBaseRobot.ROS2Interface` _output_get)))))