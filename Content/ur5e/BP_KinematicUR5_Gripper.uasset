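; Kinematic UR5e robot arm with a Robotiq 2F-140 gripper child actor and a ROS 2 interface.
; The construction script links six joints into a chain from Base to Wrist3 and registers them in the Joints map under snake_case joint names.
; It also replaces the ROS 2 component's interface with a new UR5eRobotInterface, carrying over its Robot reference, and caches the gripper actor.
; The event graph holds no logic.
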(fn `UserConstructionScript`
  (bind _elbowjoint (`self.ElbowJoint`))
  (bind _wrist1joint (`self.Wrist1Joint`))
  (bind _wrist2joint (`self.Wrist2Joint`))
  (bind _wrist3joint (`self.Wrist3Joint`))
  (bind _shoulderliftjoint (`self.ShoulderLiftJoint`))
  (bind _shoulderpanjoint (`self.ShoulderPanJoint`))
  (bind _joints (`self.Joints`))
  (bind _ros2interfacecomponent (`self.ROS2InterfaceComponent`))
  (bind _ros2interface (`RRRobotROS2InterfaceComponent.ROS2Interface` _ros2interfacecomponent))
  (`|ExecutionSequence`
    (:`then_0`
      (set `RRJointComponent.ParentLink` (`self.Base`) _shoulderpanjoint)
      (set `RRJointComponent.ChildLink` (`self.Shoulder`) _shoulderpanjoint))
    (:`then_1`
      (set `RRJointComponent.ParentLink` (`self.Shoulder`) _shoulderliftjoint)
      (set `RRJointComponent.ChildLink` (`self.Upper`) _shoulderliftjoint))
    (:`then_2`
      (set `RRJointComponent.ParentLink` (`self.Upper`) _elbowjoint)
      (set `RRJointComponent.ChildLink` (`self.Forearm`) _elbowjoint))
    (:`then_3`
      (`BlueprintMapLibrary.Map_Add` _joints "shoulder_pan_joint" (`self.ShoulderPanJoint`))
      (`BlueprintMapLibrary.Map_Add` _joints "shoulder_lift_joint" (`self.ShoulderLiftJoint`))
      (`BlueprintMapLibrary.Map_Add` _joints "elbow_joint" (`self.ElbowJoint`))
      (`BlueprintMapLibrary.Map_Add` _joints "wrist_1_joint" (`self.Wrist1Joint`))
      (`BlueprintMapLibrary.Map_Add` _joints "wrist_2_joint" (`self.Wrist2Joint`))
      (`BlueprintMapLibrary.Map_Add` _joints "wrist_3_joint" (`self.Wrist3Joint`)))
    (:`then_4`
      (set `RRJointComponent.ParentLink` (`self.Forearm`) _wrist1joint)
      (set `RRJointComponent.ChildLink` (`self.Wrist1`) _wrist1joint))
    (:`then_5`
      (set `RRJointComponent.ParentLink` (`self.Wrist1`) _wrist2joint)
      (set `RRJointComponent.ChildLink` (`self.Wrist2`) _wrist2joint))
    (:`then_6`
      (set `RRJointComponent.ParentLink` (`self.Wrist2`) _wrist3joint)
      (set `RRJointComponent.ChildLink` (`self.Wrist3`) _wrist3joint))
    (:`then_7`
      ;[1 1 1] Set ROS 2 topic name
      (if (`KismetSystemLibrary.IsValid` _ros2interface)
        _
        (else
          _))
      (bind _returnvalue (`|GenericCreateObject` "/Game/Blueprints/UR5eRobotInterface.UR5eRobotInterface_C"))
      (set `RRRobotROS2Interface.Robot` (`RRRobotROS2Interface.Robot` _ros2interface) _returnvalue)
      (set `self.ROS2Interface` _returnvalue)
      (set `RRRobotROS2InterfaceComponent.ROS2Interface` _returnvalue _ros2interfacecomponent))
    (:`then_8`
      (bind _asrobotiq_2f_140_base_blueprint (cast `/Game/ur5e/Robotiq_2F_140_base/Robotiq_2F_140_base_Blueprint` (`ChildActorComponent.ChildActor` (`self.gripper`))))
      (set `self.GripperActor` _asrobotiq_2f_140_base_blueprint))))